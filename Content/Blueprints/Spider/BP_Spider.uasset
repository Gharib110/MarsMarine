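; BP_Spider is an alien enemy that chases the player marine and attacks in melee.
; BeginPlay loops AIMoveTo on the player, while Tick pauses movement to play the attack montage within range.
; ApplyDamageToPlayer deals the hit but has no caller in this Blueprint.
; Damage lowers health; at zero the spider stops, disables collision, registers its death with the game mode, then after a delay destroys itself and increments marine kills.
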(event EventBeginPlay
  (bind _asbp_marine (Utilities|Casting|CastToBP_Marine (Game|GetPlayerCharacter 0)))
  (Variables|Default|SetAs%20BP%20Marine _asbp_marine)
  (AI|AIMoveTo self "0, 0, 0" (Game|GetPlayerCharacter 0) 5.0 false :!label _label
    (:OnSuccess
      _)
    (:OnFail
      _))
  (Utilities|FlowControl|Delay 0.2)
  (goto _label))

(event Collision|EventActorBeginOverlap
  (params (OtherActor :type Actor%20Object%20Reference)))

(event EventTick
  (params (DeltaSeconds :type Float%20%28single-precision%29))
  (bind _as_bp_marine (Variables|Default|GetAs%20BP%20Marine))
  (Utilities|IsValid _as_bp_marine
    (:Is%20Valid
      (if (Math|Boolean|ANDBoolean (CallFunction|IsWithinAttackRange) (not (CallFunction|IsAttackingPlaying)) (CallFunction|IsAlive) (Default|IsAlive _as_bp_marine))
        (Components|Activation|Deactivate (Variables|Character|GetCharacterMovement))
        (Animation|Montage|PlayMontage (Variables|Character|GetMesh) "/Game/Characters/Enemy_Great_Spider/Animations/Spider_Attack_Montage1.Spider_Attack_Montage1"
          (:OnCompleted
            (Components|Activation|Activate (Variables|Character|GetCharacterMovement) false)))))))

(event Game|Damage|EventAnyDamage
  (params (Damage :type Float%20%28single-precision%29) (DamageType :type Damage%20Type%20Object%20Reference) (InstigatedBy :type Controller%20Object%20Reference) (DamageCauser :type Actor%20Object%20Reference))
  (bind _output_get (Variables|Default|SetAlienHealth (Math|Float|Clamp(Float) (- (Variables|Default|GetAlienHealth) Damage) 0.0 1e+02)))
  (if (== _output_get 0.0)
    (CallFunction|KillAI)
    (Utilities|FlowControl|Delay 2.0)
    (Actor|DestroyActor)
    (bind _asbp_marine (Utilities|Casting|CastToBP_Marine (Game|GetPlayerCharacter 0)))
    (Default|IncreaseKills _asbp_marine)))

(fn ConstructionScript)

(fn IsWithinAttackRange
  (return (< (Transformation|GetDistanceTo (Game|GetPlayerCharacter 0)) (Variables|Default|GetAttackRange))))

(fn IsAttackingPlaying
  (return (Animation|Montage|MontageIsPlaying (Components|SkeletalMesh|GetAnimInstance (Variables|Character|GetMesh)) "/Game/Characters/Enemy_Great_Spider/Animations/Spider_Attack_Montage1.Spider_Attack_Montage1")))

(fn ApplyDamagetoPlayer
  (if (CallFunction|IsAlive)
    (Game|Damage|ApplyDamage (Game|GetPlayerCharacter 0) (Variables|Default|GetDamagePerHit) 0 0)))

(fn KillAI
  (Variables|Default|SetIsDead true)
  (CallFunction|DeactivateAlienMovement)
  (Components|Activation|Deactivate (Variables|Character|GetCharacterMovement))
  (Collision|SetActorEnableCollision false)
  (bind _asbp_marine_game_mode (Utilities|Casting|CastToBP_Marine_GameMode (Game|GetGameMode)))
  (Default|RegisterAlienDeath _asbp_marine_game_mode self))

(fn IsAlive
  (return (not (Variables|Default|GetIsDead))))

(fn DeactivateAlienMovement
  (Components|Movement|StopMovementImmediately (Variables|Character|GetCharacterMovement))
  (return))